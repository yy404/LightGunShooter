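; BP_CameraPawn is a pawn that travels along the spline of a referenced BPSpline actor, apparently as a camera fly-through.
; SpaceBar calls Start and Backspace calls Stop, which open and close a gate on Tick.
; While the gate is open, each tick adds Speed to Distance, independent of delta time, and moves the pawn to that world-space spline location without changing rotation.
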(event Custom|Stop
  (Utilities|FlowControl|Gate true) ; enters at Close
)

(event Custom|Start
  (Utilities|FlowControl|Gate true) ; enters at Open
)

(event EventTick
  (params (DeltaSeconds :type Float%20%28single-precision%29))
  (Utilities|FlowControl|Gate true
    (:Exit
      (Variables|Default|Setdistance (+ (Variables|Default|Getdistance) (Variables|Default|Getspeed)))
      (Transformation|SetActorLocation (Spline|GetLocationatDistanceAlongSpline (Variables|/Game/BP_Spline.BP_Spline_C|GetSpline (Variables|Default|GetBP_Spline)) (Variables|Default|Getdistance) "World") false false))))

(event Input|KeyboardEvents|SpaceBar
  (params (Key :type Key%20Structure :default "None"))
  (:Pressed
    (CallFunction|Start)))

(event Input|KeyboardEvents|Backspace
  (params (Key :type Key%20Structure :default "None"))
  (:Pressed
    (CallFunction|Stop)))

(fn ConstructionScript)